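; Level exit doorway that opens once the game mode's enemy count reaches zero and sends the player to a random next level.
; BeginPlay runs a custom Constructor that closes the door, picks the destination from the game instance's random stream and sets the marker widget's origin.
; Tick polls the enemy count; opening changes material and light, shows the marker and adds audio.
; A player hit on the open door saves health and score plus a bonus, then loads the destination.
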(event `self.ReceiveBeginPlay`
  ;[1 1 1] A workaround to make sure the constructor is always called
  (`self.Constructor`))

(event `self.ReceiveHit`
  (params (MyComp :type "PrimitiveComponent Object Reference") (Other :type "Actor Object Reference") (OtherComp :type "PrimitiveComponent Object Reference") (bSelfMoved :type Boolean) (HitLocation :type "Vector Structure") (HitNormal :type "Vector Structure") (NormalImpulse :type "Vector Structure") (Hit :type "HitResult Structure (by ref)"))
  ;[1 1 1] Open next level on Player Hit when open
  (if (`self.isOpen`)
    (if (`KismetStringLibrary.Contains` (`KismetSystemLibrary.GetObjectName` Other) "BP_Player")
      (bind _asbp_player (cast `/Game/_Game/Assets/Player/BP_Player` (`GameplayStatics.GetPlayerPawn` 0)))
      (`/Game/_Game/Assets/Player/BP_Player.SavePlayerInfo` _asbp_player (`/Game/_Game/Assets/Player/BP_Player.Health` _asbp_player) (+ (`/Game/_Game/Assets/Player/BP_Player.Score` _asbp_player) 1000))
      (`GameplayStatics.OpenLevel` (`self.destination`)))))

(event `self.ReceiveTick`
  (params (DeltaSeconds :type "Float (single-precision)"))
  ;[1 1 1] Every tick check if the door should be opened
  (bind _asbp_gamemode (cast `/Game/_Game/BP_Gamemode` (`GameplayStatics.GetGameMode`)))
  (bind _enemycount (`/Game/_Game/BP_Gamemode.EnemyCount` _asbp_gamemode))
  (`KismetSystemLibrary.PrintString` (`KismetStringLibrary.Conv_IntToString` _enemycount))
  (if (and (<= _enemycount 0) (not (`self.isOpen`)))
    (`self.OpenDoor`)))

(fn `CloseDoor`
  (bind _spotlight (`self.SpotLight`))
  (set `self.isOpen` false)
  (`PrimitiveComponent.SetMaterial` (`self.StaticMeshComponent`) 0 (`self.ClosedMat`))
  (`LightComponent.SetIntensity` _spotlight 8.0)
  (`LightComponent.SetLightColor` _spotlight (struct :`R` 0.002934 :`G` 0.039423 :`B` 1.0 :`A` 1.0) true))

(fn `Constructor`
  (`KismetSystemLibrary.PrintText` "Construction here")
  (`self.CloseDoor`)
  (`self.setDestination`)
  (`ActorComponent.SetComponentTickEnabled` (`self.StaticMeshComponent`) false)
  (bind _asw_marker (cast `/Game/_Game/Assets/Healthbar/W_Marker` (`WidgetComponent.GetWidget` (`self.Widget`))))
  (set `/Game/_Game/Assets/Healthbar/W_Marker.OriginLocation` (`self.K2_GetActorLocation`) _asw_marker))

(fn `getLevelCount`
  (returns (levelCount :type Integer))
  (bind _asbp_game_instance (cast `/Game/_Game/BP_GameInstance` (`GameplayStatics.GetGameInstance`))
    (:`then`
      (return (`/Game/_Game/BP_GameInstance.AvailableLevelCount` _asbp_game_instance)))
    (:`CastFailed`
      (`KismetSystemLibrary.PrintText` "Cast to BP_GameInstance failed")
      (return -1))))

(fn `OpenDoor`
  (bind _spotlight (`self.SpotLight`))
  (set `self.isOpen` true)
  (`PrimitiveComponent.SetMaterial` (`self.StaticMeshComponent`) 0 (`self.OpenMat`))
  (`LightComponent.SetIntensity` _spotlight 40.0)
  (`LightComponent.SetLightColor` _spotlight (struct :`R` 0.933388 :`G` 0.147295 :`B` 1.0 :`A` 1.0) true)
  (`Widget.SetVisibility` (`WidgetComponent.GetWidget` (`self.Widget`)) "Visible")
  (`AddComponent|NODE_AddAudioComponent-0`))

(fn `setDestination`
  (locals (destinationString :type String) (levelCount :type Integer))
  (bind _levelcount (`self.getLevelCount`))
  (bind _output_get (set `local.levelCount` _levelcount))
  (bind _result (`/Engine/EditorBlueprintResources/StandardMacros.DecrementInt` _output_get)
    (:`  `
      (bind _asbp_game_instance (cast `/Game/_Game/BP_GameInstance` (`GameplayStatics.GetGameInstance`)))
      (bind _output_get_2 (set `local.destinationString` "level"))
      (bind _output_get_3 (set `local.destinationString` (`KismetStringLibrary.BuildString_Int` _output_get_2 "" (`KismetMathLibrary.RandomIntegerInRangeFromStream` (`/Game/_Game/BP_GameInstance.Rnd` _asbp_game_instance) 0 _result))))
      (bind _output_get_4 (set `self.destination` (`KismetStringLibrary.Conv_StringToName` _output_get_3)))
      (`KismetSystemLibrary.PrintString` (`KismetStringLibrary.Conv_NameToString` _output_get_4))
      (return))))

(fn `UserConstructionScript`)