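; Base destructible actor that shatters its static mesh into a Chaos geometry collection on the first damage not caused by itself.
; Destruction swaps in a simulated collection that ignores pawns and vehicles, and damages the parent actor.
; A radial impulse from below scatters the pieces, which later ignore world collision before the actor is destroyed.
; OnDestroyed calls AfterBreak, an empty function here.
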(event `self.ReceiveAnyDamage`
  (params (Damage :type "Float (single-precision)") (DamageType :type "DamageType Object Reference") (InstigatedBy :type "Controller Object Reference") (DamageCauser :type "Actor Object Reference"))
  (if (not (== DamageCauser self))
    (`/Engine/EditorBlueprintResources/StandardMacros.DoOnce` false
      (:`Completed`
        (bind _collectioncomponent (`self.Destruction`))
        (`ActorComponent.K2_DestroyComponent` (`self.StaticMeshComponent`))
        (`PrimitiveComponent.AddRadialImpulse` _collectioncomponent (+ (`self.K2_GetActorLocation`) (0.0 0.0 -80.0)) (`self.ImpulseRadius`) (`self.ImpulseStrength`) "RIF_Linear" true)
        (`KismetSystemLibrary.Delay` 3.0)
        (`PrimitiveComponent.SetCollisionResponseToChannel` _collectioncomponent "ECC_WorldDynamic" "ECR_Ignore")
        (`PrimitiveComponent.SetCollisionResponseToChannel` _collectioncomponent "ECC_WorldStatic" "ECR_Ignore")
        (`KismetSystemLibrary.Delay` 5.0)
        (`self.K2_DestroyActor`)))))

(event `self.ReceiveBeginPlay`
  (add `self.OnDestroyed` (delegate `OnDestroyed_Event`)))

(event `OnDestroyed_Event` :!signature `self.OnDestroyed`
  (params (DestroyedActor :type "Actor Object Reference"))
  (`self.AfterBreak`))

(fn `AfterBreak`
  (return))

(fn `Destruction`
  (returns (CollectionComponent :type "GeometryCollectionComponent Object Reference"))
  (`PrimitiveComponent.SetCollisionEnabled` (`self.StaticMeshComponent`) "NoCollision")
  (`SceneComponent.SetVisibility` (`self.StaticMeshComponent`) false false)
  (bind _returnvalue (`AddComponent|NODE_AddGeometryCollectionComponent-0`))
  (`GeometryCollectionComponent.SetRestCollection` _returnvalue (`self.RestCollection`) false)
  (`PrimitiveComponent.SetCollisionEnabled` _returnvalue "PhysicsOnly")
  (`PrimitiveComponent.SetCollisionObjectType` _returnvalue "ECC_Destructible")
  (`PrimitiveComponent.SetCollisionResponseToAllChannels` _returnvalue "ECR_Block")
  (`PrimitiveComponent.SetCollisionResponseToChannel` _returnvalue "ECC_GameTraceChannel1" "ECR_Ignore")
  (`PrimitiveComponent.SetCollisionResponseToChannel` _returnvalue "ECC_Pawn" "ECR_Ignore")
  (`PrimitiveComponent.SetCollisionResponseToChannel` _returnvalue "ECC_Vehicle" "ECR_Ignore")
  (`PrimitiveComponent.SetSimulatePhysics` _returnvalue true)
  (set `GeometryCollectionComponent.DamageThreshold` (`|MakeArray` 1.0 1.0 1.0 :!type "Float (single-precision)") _returnvalue)
  (`GameplayStatics.ApplyDamage` (`self.GetParentActor`) 20.0)
  (return _returnvalue))

(fn `UserConstructionScript`)