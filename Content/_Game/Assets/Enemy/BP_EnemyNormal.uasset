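; BP_EnemyNormal is a zombie enemy that chases the player, punches, and registers itself in BP_Gamemode's EnemyCount while alive.
; A self-restarting AI MoveTo loop plays the attack montage on arrival and retries after failure.
; HitDetect sphere-traces at the right hand to damage BP_Player, with no caller in this file.
; Incoming damage is throttled by a DoOnce, flashes the material, and at zero health triggers a death montage before destruction.
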(event `OnDestroyed_Event` :!signature `self.OnDestroyed`
  (params (DestroyedActor :type "Actor Object Reference"))
  ;[1 1 1] On Destroy event
  (bind _asbp_gamemode (cast `/Game/_Game/BP_Gamemode` (`GameplayStatics.GetGameMode`)))
  (set `/Game/_Game/BP_Gamemode.EnemyCount` (- (`/Game/_Game/BP_Gamemode.EnemyCount` _asbp_gamemode) 1) _asbp_gamemode))

(event `self.ReceiveBeginPlay`
  ;[1 1 1] Start Enemy
  (`self.ChasePlayer`)
  (add `self.OnDestroyed` (delegate `OnDestroyed_Event`))
  (bind _asbp_gamemode (cast `/Game/_Game/BP_Gamemode` (`GameplayStatics.GetGameMode`)))
  (set `/Game/_Game/BP_Gamemode.EnemyCount` (+ (`/Game/_Game/BP_Gamemode.EnemyCount` _asbp_gamemode) 1) _asbp_gamemode))

(event `self.ReceiveTick`
  (params (DeltaSeconds :type "Float (single-precision)")))

(event `ChasePlayer`
  ;[1 1 1] Chase Player
  (`self.AISpeed`)
  (`|AIMoveTo` self (0.0 0.0 0.0) (`GameplayStatics.GetPlayerCharacter` 0) 0.1
    (:`OnSuccess`
      (`self.Attack`)
      (`Timeline|Attacking Delay` :!via `PlayFromStart`
        (:`Finished`
          _)))
    (:`OnFail`
      (`KismetSystemLibrary.Delay` 0.2)))
  (`self.ChasePlayer`))

(event `AISpeed`
  ;[1 1 1] Speed of movement
  (set `CharacterMovementComponent.MaxWalkSpeed` (* 300.0 (`self.MovementSpeed`)) (`self.CharacterMovement`)))

(event `Attack`
  ;[1 1 1] Animation Attak
  (if (not (`self.IsDead`))
    (`|PlayMontage` (`self.Mesh`) "/Game/_Game/Assets/Enemy/enemy-lis/animations/Zombie_Punching_Montage.Zombie_Punching_Montage")))

(event `On Death`
  ;[1 1 1] On Death
  (set `self.IsDead` true)
  (`self.SetActorEnableCollision` self false)
  (`CharacterMovementComponent.DisableMovement` (`self.CharacterMovement`))
  (`|PlayMontage` (`self.Mesh`) "/Game/_Game/Assets/Enemy/enemy-lis/animations/Dying_Anim_Montage.Dying_Anim_Montage"
    (:`then`
      (`KismetSystemLibrary.Delay` 2.0)
      (`self.K2_DestroyActor`))))

(event `self.ReceiveAnyDamage`
  (params (Damage :type "Float (single-precision)") (DamageType :type "DamageType Object Reference") (InstigatedBy :type "Controller Object Reference") (DamageCauser :type "Actor Object Reference"))
  ;[1 1 1] Recived dmg
  (`/Engine/EditorBlueprintResources/StandardMacros.DoOnce` false :!label _label
    (:`Completed`
      (set `self.Health` (- (`self.Health`) Damage))
      (`self.FlashWhenHit`)
      (if (<= (`self.Health`) 0.0)
        (`self.On Death`)
        (else
          (`KismetSystemLibrary.PrintText` (`KismetTextLibrary.Conv_DoubleToText` (`self.Health`) "HalfToEven"))
          (`KismetSystemLibrary.Delay` 0.4)
          (goto _label :!via `Reset`))))))

(event `FlashWhenHit`
  ;[1 1 1] Flash When Hit Effect
  (`PrimitiveComponent.SetMaterial` (`self.Mesh`) 0 "/Game/_Game/Assets/Enemy/enemy-lis/mesh/Glow-Enemy-Material.Glow-Enemy-Material")
  (`KismetSystemLibrary.Delay` 0.1)
  (`PrimitiveComponent.SetMaterial` (`self.Mesh`) 0 "/Game/_Game/Assets/Enemy/enemy-lis/mesh/Untitled_Material.Untitled_Material"))

(fn `Hit detect`
  (bind _returnvalue (`SceneComponent.GetSocketLocation` (`self.Mesh`) "hand_r"))
  (bind _outhit (`KismetSystemLibrary.SphereTraceSingleForObjects` :`Start` _returnvalue :`End` _returnvalue :`Radius` 30.0 :`ObjectTypes` (`|MakeArray` "ObjectTypeQuery3" :!type "EObjectTypeQuery Enum") :`DrawDebugType` "ForDuration"))
  (bind _asbp_player (cast `/Game/_Game/Assets/Player/BP_Player` (`.HitActor` (`GameplayStatics.BreakHitResult` _outhit))))
  (`GameplayStatics.ApplyDamage` _asbp_player (`self.Dmg`)))

(fn `UserConstructionScript`)