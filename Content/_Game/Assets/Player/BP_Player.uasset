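; Player character with cursor-facing rotation, sword attacks, damage flash, death screen and pause menu.
; Enhanced Input drives world-axis movement, montage attacks and a timeline-driven roll whose distance depends on stamina, which regenerates from Tick.
; HitDetect sphere-traces between sword sockets to damage pawns, while incoming damage is gated by a short DoOnce cooldown.
; BeginPlay creates the health bar, loads saved health and score, and branches audio on score.
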(event `self.ReceiveBeginPlay`
  (bind _returnvalue (`GameplayStatics.GetPlayerController` 0))
  ;[1 1 1] Game start
  (set `self.Health` (`self.Max_Health`))
  (set `self.Stamina` (`self.MaxStamina`))
  (bind _returnvalue_2 (`|CreateWidget` "/Game/_Game/Assets/Healthbar/WBP_Healthbar.WBP_Healthbar_C" _returnvalue))
  (`UserWidget.AddToViewport` _returnvalue_2 0)
  (`WidgetBlueprintLibrary.SetInputMode_GameAndUIEx` _returnvalue null "DoNotLock" false)
  (bind (_health _score) (`self.LoadPlayerInfo`))
  (set `self.Health` _health)
  (set `self.Score` _score)
  (`AddComponent|NODE_AddAudioComponent-0`)
  (`KismetSystemLibrary.Delay` 2.3)
  (if (>= (`self.Score`) 1000000)
    (bind _returnvalue_3 (`AddComponent|NODE_AddAudioComponent-8`))
    (set `self.2DSound` _returnvalue_3)
    (else
      (bind _returnvalue_4 (`AddComponent|NODE_AddAudioComponent-7`))
      (set `self.2DSound` _returnvalue_4))))

(event `self.ReceiveTick`
  (params (DeltaSeconds :type "Float (single-precision)"))
  ;[1 1 1] Look at Cursor
  (`self.Stamina Regeneration`)
  (bind _output_get (set `self.Delta Time` DeltaSeconds))
  (if (not (`self.InRoll`))
    (`self.K2_SetActorRotation` (`KismetMathLibrary.RInterpTo_Constant` (`self.K2_GetActorRotation`) (stale `/Game/_Game/BP_Interface.Look At` _output_get) _output_get (`self.Speed Rotation`)))))

(event `/Game/_Game/BP_Interface.Look At`
  (params (Target :type "Vector Structure"))
  (bind (_returnvalue_x _returnvalue_y) (`KismetMathLibrary.BreakVector` (`self.K2_GetActorLocation`)))
  ;[1 1 1] Look at Cursor
  (bind _output_get (set `self.TargetRotation` (`KismetMathLibrary.FindLookAtRotation` (`KismetMathLibrary.MakeVector` _returnvalue_x _returnvalue_y) (`KismetMathLibrary.MakeVector` Target_X Target_Y)))))

(event `self.ReceiveAnyDamage`
  (params (Damage :type "Float (single-precision)") (DamageType :type "DamageType Object Reference") (InstigatedBy :type "Controller Object Reference") (DamageCauser :type "Actor Object Reference"))
  ;[1 1 1] Recived dmg
  (`/Engine/EditorBlueprintResources/StandardMacros.DoOnce` false :!label _label
    (:`Completed`
      (`self.FlashWhenHit`)
      (set `self.Health` (- (`self.Health`) Damage))
      (if (<= (`self.Health`) 0.0)
        (bind _returnvalue (`|CreateWidget` "/Game/_Game/Assets/DeathScreen.DeathScreen_C"))
        (`UserWidget.AddToViewport` _returnvalue 0)
        (`WidgetBlueprintLibrary.SetInputMode_UIOnlyEx` (`GameplayStatics.GetPlayerController` 0) null)
        (`AudioComponent.Stop` (`self.2DSound`))
        (`AddComponent|NODE_AddAudioComponent-3`)
        (else
          (`AddComponent|NODE_AddAudioComponent-4`)
          (`KismetSystemLibrary.Delay` 0.4)
          (goto _label :!via `Reset`))))))

(event `FlashWhenHit`
  ;[1 1 1] Flash When Hit Effect
  (`PrimitiveComponent.SetMaterial` (`self.Mesh`) 0 "/Game/_Game/Assets/Player/MeshSkeleton/Hitplayer.Hitplayer")
  (`KismetSystemLibrary.Delay` 0.2)
  (`PrimitiveComponent.SetMaterial` (`self.Mesh`) 0 "/Game/_Game/Assets/Player/MeshSkeleton/player_Material.player_Material"))

(event `Stamina Regeneration`
  ;[1 1 1] Stamina Regen
  (if (not (>= (`self.Stamina`) 100.0))
    (`KismetSystemLibrary.Delay` (`self.StaminaRegenSpeed`))
    (set `self.Stamina` (+ (`self.Stamina`) (`self.StaminaRegen`)))
    (`KismetSystemLibrary.PrintText` (`KismetTextLibrary.Conv_DoubleToText` (`self.Stamina`) "HalfToEven"))))

(event `EnhancedInput|/Game/_Game/Assets/Player/Input/PlayerIAMovement`
  (params (ActionValue :type "Vector2D Structure") (ElapsedSeconds :type "Float (double-precision)") (TriggeredSeconds :type "Float (double-precision)") (InputAction :type "InputAction Object Reference" :default "/Game/_Game/Assets/Player/Input/PlayerIAMovement.PlayerIAMovement"))
  (bind _returnvalue (`KismetMathLibrary.MakeRotator` 0.0))
  ;[1 1 1] EnhancedInput Movement
  (:`Triggered`
    (if (not (`self.InRoll`))
      (`|ExecutionSequence`
        (:`then_0`
          (`self.AddMovementInput` (`KismetMathLibrary.GetForwardVector` _returnvalue) ActionValue_Y))
        (:`then_1`
          (`self.AddMovementInput` (`KismetMathLibrary.GetRightVector` _returnvalue) ActionValue_X))))))

(event `EnhancedInput|/Game/_Game/Assets/Player/Input/PlayerIAJump`
  (params (ActionValue :type Boolean) (ElapsedSeconds :type "Float (double-precision)") (TriggeredSeconds :type "Float (double-precision)") (InputAction :type "InputAction Object Reference" :default "/Game/_Game/Assets/Player/Input/PlayerIAJump.PlayerIAJump"))
  (bind _stamina (`self.Stamina`))
  (bind (_velocity_x _velocity_y _velocity_z) (`KismetMathLibrary.BreakVector` (`MovementComponent.Velocity` (`self.CharacterMovement`))))
  ;[1 1 1] Skok w bok
  (:`Completed`
    (if (`self.InRoll`)
      _
      (elif (> (`KismetMathLibrary.VSize` (`MovementComponent.Velocity` (`self.CharacterMovement`))) 1.0)
        (if (not (<= (`self.Stamina`) 0.0))
          (`self.Calculate Move Distance`)
          (set `self.InRoll` true)
          (`self.Set Rotation On Roll`)
          (bind _returnvalue (`self.PlayAnimMontage` "/Game/_Game/Assets/Player/Animations/SRoll_Montage.SRoll_Montage"))
          (bind (_direction _distance_multiplayer) (`Timeline|Timeline` :!via `PlayFromStart`)
            (:`Update`
              (bind (_returnvalue_x _returnvalue_y) (`KismetMathLibrary.BreakVector` (* (`self.GetActorForwardVector`) (* _distance_multiplayer (`self.MoveDistance`)))))
              (set `MovementComponent.Velocity` (`KismetMathLibrary.MakeVector` _returnvalue_x _returnvalue_y _velocity_z) (`self.CharacterMovement`))
              (`KismetSystemLibrary.Delay` _returnvalue)
              (set `self.InRoll` false)
              (if (< _stamina 40.0)
                (set `self.Stamina` 0.0)
                (else
                  (set `self.Stamina` (- _stamina 40.0))
                  (`KismetSystemLibrary.PrintText` (`KismetTextLibrary.Conv_DoubleToText` _stamina "HalfToEven")))))))))))

(event `Calculate Move Distance`
  (bind _returnvalue (* (* (`self.Stamina`) 0.01) (`self.MoveDistance`)))
  ;[1 1 1] Calculate Move Distance
  (if (<= (`self.Stamina`) 40.0)
    (if (<= (`self.Stamina`) 20.0)
      (set `self.MoveDistance` 600.0)
      (elif (<= _returnvalue 750.0)
        (set `self.MoveDistance` 750.0)
        (else
          (set `self.MoveDistance` _returnvalue))))
    (else
      (set `self.MoveDistance` 1150.0))))

(event `Set Rotation On Roll`
  (bind (_returnvalue_roll _returnvalue_pitch _returnvalue_yaw) (`KismetMathLibrary.BreakRotator` (`KismetMathLibrary.Conv_VectorToRotator` (`CharacterMovementComponent.GetLastUpdateVelocity` (`self.CharacterMovement`)))))
  ;[1 1 1] Set Rotation On Roll
  (`self.K2_SetActorRotation` (`KismetMathLibrary.MakeRotator` 0.0 0.0 _returnvalue_yaw)))

(event `EnhancedInput|/Game/_Game/Assets/Player/Input/Attack`
  (params (ActionValue :type Boolean) (ElapsedSeconds :type "Float (double-precision)") (TriggeredSeconds :type "Float (double-precision)") (InputAction :type "InputAction Object Reference" :default "/Game/_Game/Assets/Player/Input/Attack.Attack"))
  ;[1 1 1] Attak
  (:`Completed`
    (if (not (`self.InRoll`))
      (`/Engine/EditorBlueprintResources/StandardMacros.DoOnce` false :!label _label
        (:`Completed`
          (bind _returnvalue (`self.PlayAnimMontage` "/Game/_Game/Assets/Player/Animations/Attack1_Montage.Attack1_Montage"))
          (`KismetSystemLibrary.Delay` _returnvalue)
          (goto _label :!via `Reset`))))))

(event `EnhancedInput|/Game/_Game/Assets/Player/Input/PauseGame`
  (params (ActionValue :type Boolean) (ElapsedSeconds :type "Float (double-precision)") (TriggeredSeconds :type "Float (double-precision)") (InputAction :type "InputAction Object Reference" :default "/Game/_Game/Assets/Player/Input/PauseGame.PauseGame"))
  (bind _returnvalue (`GameplayStatics.GetPlayerController` 0))
  (bind _pausemenuwidget (`self.pausemenuwidget`))
  ;[1 1 1] Pause
  (:`Completed`
    (if (not (`self.IsPauseMenuOpen`))
      (set `self.IsPauseMenuOpen` true)
      (bind _returnvalue_2 (`|CreateWidget` "/Game/_Game/Blueprints/PauseMenu.PauseMenu_C" _returnvalue))
      (bind _output_get (set `self.pausemenuwidget` _returnvalue_2))
      (`UserWidget.AddToViewport` _output_get 0)
      (`WidgetBlueprintLibrary.SetInputMode_GameAndUIEx` _returnvalue _pausemenuwidget)
      (`GameplayStatics.SetGamePaused` true)
      (else
        (set `self.IsPauseMenuOpen` false)
        (`Widget.RemoveFromParent` _pausemenuwidget)
        (`GameplayStatics.SetGamePaused` false)))))

(fn `Hit detect`
  (bind _sword (`self.Sword`))
  (bind _outhit (`KismetSystemLibrary.SphereTraceSingleForObjects` :`Start` (`SceneComponent.GetSocketLocation` _sword "Start") :`End` (`SceneComponent.GetSocketLocation` _sword "End") :`Radius` 15.0 :`ObjectTypes` (`|MakeArray` "ObjectTypeQuery3" :!type "EObjectTypeQuery Enum") :`DrawDebugType` "ForDuration"))
  (bind _aspawn (cast `Pawn` (`.HitActor` (`GameplayStatics.BreakHitResult` _outhit))))
  (`GameplayStatics.ApplyDamage` _aspawn (`self.Dmg`)))

(fn `LoadPlayerInfo`
  (returns (Health :type "Float (double-precision)") (Score :type Integer))
  (bind _max_health (`self.Max_Health`))
  (bind _returnvalue (`GameplayStatics.DoesSaveGameExist` "PlayerInfo"))
  (if _returnvalue
    (bind _returnvalue_2 (`GameplayStatics.LoadGameFromSlot` "PlayerInfo"))
    (bind _output_get (set `self.PlayerInfoo` _returnvalue_2))
    (bind _assave_player_info (cast `/Game/_Game/Blueprints/SavePlayerInfo` _output_get)
      (:`then`
        (return (`/Game/_Game/Blueprints/SavePlayerInfo.Health` _assave_player_info) (`/Game/_Game/Blueprints/SavePlayerInfo.Score` _assave_player_info)))
      (:`CastFailed`
        (return _max_health 0)))
    (else
      (return _max_health 0))))

(fn `SavePlayerInfo`
  (params (Health :type "Float (double-precision)") (Score :type Integer))
  (bind _returnvalue (`GameplayStatics.CreateSaveGameObject` "/Game/_Game/Blueprints/SavePlayerInfo.SavePlayerInfo_C"))
  (bind _output_get (set `self.PlayerInfo` _returnvalue))
  (bind _assave_player_info (cast `/Game/_Game/Blueprints/SavePlayerInfo` _output_get))
  (set `/Game/_Game/Blueprints/SavePlayerInfo.Health` Health _assave_player_info)
  (set `/Game/_Game/Blueprints/SavePlayerInfo.Score` Score _assave_player_info)
  (bind _returnvalue_2 (`GameplayStatics.SaveGameToSlot` (`self.PlayerInfo`) "PlayerInfo"))
  (if _returnvalue_2
    (`KismetSystemLibrary.PrintString` "Saved")
    (else
      (`KismetSystemLibrary.PrintString` "Error: Not saved"))))

(fn `UserConstructionScript`)