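; Bandage pickup Blueprint that heals the player when picked up.
; OnPickup finds the player with GetActorOfClass on BP_Player, adds HealValue to its Health, then clamps the result to MaxHealth.
; The event graph holds only disabled stub events and the construction script just calls its parent, so all of this Blueprint's own logic lives in OnPickup.
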(fn `OnPickup`
  (bind _returnvalue (`GameplayStatics.GetActorOfClass` "/Game/_Game/Assets/Player/BP_Player.BP_Player_C"))
  (bind _output_get (set `/Game/_Game/Assets/Player/BP_Player.Health` (+ (`self.HealValue`) (`/Game/_Game/Assets/Player/BP_Player.Health` _returnvalue)) _returnvalue))
  (bind _max_health (`/Game/_Game/Assets/Player/BP_Player.Max_Health` _returnvalue))
  (if (> _output_get _max_health)
    (set `/Game/_Game/Assets/Player/BP_Player.Health` _max_health _returnvalue)))

(fn `UserConstructionScript`
  (`parent.UserConstructionScript`))